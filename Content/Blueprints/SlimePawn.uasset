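; Slime enemy pawn that chases the first-person player character using AI navigation.
; BeginPlay caches the player, then PathfindToPlayer runs AIMoveTo toward the player's current location and re-issues it on success or failure.
; A Tick state machine requests Moving from Idle and re-paths every tick while Moving.
; ChangeState is a stub that never sets CurrentState, and several alternative movement nodes are left unconnected.
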(event `self.ReceiveBeginPlay`
  (bind _returnvalue (`GameplayStatics.GetActorOfClass` "/Game/Blueprints/FirstPersonCharacter.FirstPersonCharacter_C"))
  (set `self.player` _returnvalue)
  (`self.Pathfind to Player`))

(event `Pathfind to Player`
  (bind _player (`self.player`))
  (`/Engine/EditorBlueprintResources/StandardMacros.IsValid` _player
    (:`Is Valid`
      (`|AIMoveTo` (`self.GetController`) self (`self.K2_GetActorLocation` _player) null
        (:`OnSuccess`
          _)
        (:`OnFail`
          _))
      (`self.Pathfind to Player`))))

(event `self.ReceiveTick`
  (params (DeltaSeconds :type "Float (single-precision)"))
  (switch `/Game/Blueprints/SlimeStates` (`self.current state`)
    (:`NewEnumerator0`
      ;[1 1 1] Transition to other states
      (if true
        (`self.Change State` "NewEnumerator1")))
    (:`NewEnumerator1`
      ;[1 1 1] State Behavior
      (`self.Pathfind to Player`))))

(fn `Change State`
  (params (`Next State` :type "/Game/Blueprints/SlimeStates Enum" :default "NewEnumerator0"))
  (bind _output_get (set `self.Next State` `Next State`))
  (switch `/Game/Blueprints/SlimeStates` _output_get))

(fn `UserConstructionScript`)