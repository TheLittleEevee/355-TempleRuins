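; Rideable minecart pawn that the player possesses to drive along a spline track.
; The construction script lays fixed-length spline mesh pieces along the spline and places the cart.
; Each tick, forward/backward input accelerates a clamped, friction-free velocity, then an Euler step advances spline distance to position and orient the cart.
; Boarding destroys the player's character; exiting spawns and possesses a new first-person character at the camera.
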(event `InputAxis|TurnRate`
  (params (AxisValue :type "Float (single-precision)"))
  ;[1 1 1] Stick Look
  (`self.AddControllerYawInput` (* AxisValue 45.0 (`GameplayStatics.GetWorldDeltaSeconds`))))

(event `self.ReceiveTick`
  (params (DeltaSeconds :type "Float (single-precision)"))
  (`self.Accelerate` DeltaSeconds)
  (`self.Euler Step` DeltaSeconds)
  (`self.Position Cart`))

(event `/Game/Blueprints/Interfaces/PlayerCanInteract.Player Wants to Interact`
  (params (Player :type "/Game/Blueprints/FirstPersonCharacter Object Reference"))
  ;[1 1 1] Get in Minecart
  (`Controller.Possess` (`self.GetController` Player) self)
  (`self.K2_DestroyActor` Player))

(event `InputAxis|Turn` :overrideparent false
  (params (AxisValue :type "Float (single-precision)"))
  ;[1 1 1] Mouse Look
  (`self.AddControllerYawInput` AxisValue))

(event `InputAxis|LookUp` :overrideparent false
  (params (AxisValue :type "Float (single-precision)"))
  ;[1 1 1] Mouse Look
  (`self.AddControllerPitchInput` AxisValue))

(event `InputAction|Minecart Forward`
  (params (Key :type "Key Structure"))
  (:`Pressed`
    (set `self.Player Wants to move Forward` true))
  (:`Released`
    (set `self.Player Wants to move Forward` false)))

(event `InputAxis|LookUpRate`
  (params (AxisValue :type "Float (single-precision)"))
  ;[1 1 1] Stick Look
  (`self.AddControllerPitchInput` (* AxisValue 45.0 (`GameplayStatics.GetWorldDeltaSeconds`))))

(event `InputAction|Interact`
  (params (Key :type "Key Structure"))
  (bind _returnvalue (`SceneComponent.K2_GetComponentToWorld` (`self.Camera`)))
  ;[1 1 1] Get Out of Minecart
  (:`Pressed`
    (bind _returnvalue_2 (`|SpawnActorFromClass` "/Game/Blueprints/FirstPersonCharacter.FirstPersonCharacter_C" (`KismetMathLibrary.MakeTransform` (.location _returnvalue) (`KismetMathLibrary.MakeRotator` 0.0 0.0 (.yaw (.rotation _returnvalue)))) "Undefined" "OverrideRootScale" (`self.GetOwner`) null))
    (`Controller.Possess` (`self.GetController`) _returnvalue_2)))

(event `InputAction|Minecart Backward`
  (params (Key :type "Key Structure"))
  (:`Pressed`
    (set `self.Player Wants to move Backward` true))
  (:`Released`
    (set `self.Player Wants to move Backward` false)))

(fn `Accelerate`
  (params (Dt :type "Float (double-precision)"))
  (locals (Dir :type "Float (double-precision)"))
  ;[1 1 1] Velocity = clamp(velocity + dt*acc*dir, -max, max)
  (if (`self.Player Wants to move Forward`)
    (set `local.Dir` 1.0))
  (if (`self.Player Wants to move Backward`)
    (set `local.Dir` (- (`local.Dir`) 1.0)))
  (set `self.Velocity` (`KismetMathLibrary.FClamp` (+ (`self.Velocity`) (* (`local.Dir`) Dt (`self.acceleration`))) (* -1 (`self.Max Velocity`)) (`self.Max Velocity`))))

(fn `Euler Step`
  (params (dt :type "Float (double-precision)"))
  (set `self.Position on Spline` (`KismetMathLibrary.FClamp` (+ (`self.Position on Spline`) (* (`self.Velocity`) dt)) 0.0 (`SplineComponent.GetSplineLength` (`self.Spline`)))))

(fn `Position Cart`
  (bind _spline (`self.Spline`))
  (bind _position_on_spline (`self.Position on Spline`))
  (`SceneComponent.K2_SetRelativeLocationAndRotation` (`self.Mover`) (`SplineComponent.GetLocationAtDistanceAlongSpline` _spline _position_on_spline "Local") (`SplineComponent.GetRotationAtDistanceAlongSpline` _spline _position_on_spline "Local") false false))

(fn `UserConstructionScript`
  (bind _spline (`self.Spline`))
  (`self.Position Cart`)
  (for _index (range (`KismetMathLibrary.FTrunc` (/ (`SplineComponent.GetSplineLength` (`self.Spline`)) (`self.Length of Piece`))))
    (bind _returnvalue (`AddComponent|NODE_AddSplineMeshComponent-0`))
    (bind _returnvalue_2 (* _index (`self.Length of Piece`)))
    (bind _returnvalue_3 (* (+ _index 1) (`self.Length of Piece`)))
    (`SplineMeshComponent.SetStartAndEnd` _returnvalue (`SplineComponent.GetLocationAtDistanceAlongSpline` _spline _returnvalue_2 "Local") (`KismetMathLibrary.ClampVectorSize` (`SplineComponent.GetTangentAtDistanceAlongSpline` _spline _returnvalue_2 "Local") 0.0 (`self.Length of Piece`)) (`SplineComponent.GetLocationAtDistanceAlongSpline` _spline _returnvalue_3 "Local") (`KismetMathLibrary.ClampVectorSize` (`SplineComponent.GetTangentAtDistanceAlongSpline` _spline _returnvalue_3 "Local") 0.0 (`self.Length of Piece`)) true)))