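; LED Blueprint that cycles its color state from red to green to blue and back each time Trigger fires.
; The construction script creates a dynamic material instance on the Cylinder and applies the current state's color.
; Trigger picks the next state with a Select node, then UpdateMaterialColor maps it to the "LED Color" parameter.
; An unconnected Switch-based version of the same state change remains in the event graph.
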(event `/Game/Blueprints/Interfaces/Triggerable.Trigger`
  ;[1 1 1] Change State with Select
  (set `self.Current State` (select `/Game/Blueprints/LED/LED_Color` (`self.Current State`) :`NewEnumerator0` "NewEnumerator1" :`NewEnumerator1` "NewEnumerator2" :`NewEnumerator2` "NewEnumerator0" :!type "/Game/Blueprints/LED/LED_Color Enum"))
  ;[1 1 1] Update Material
  (`self.Update Material Color`))

(fn `Update Material Color`
  (`MaterialInstanceDynamic.SetVectorParameterValue` (`self.LED Material`) "LED Color" (select `/Game/Blueprints/LED/LED_Color` (`self.Current State`) :`NewEnumerator0` (struct :`R` 1.0 :`B` 0.060824 :`A` 1.0) :`NewEnumerator1` (struct :`G` 1.0 :`B` 0.060972 :`A` 1.0) :`NewEnumerator2` (struct :`R` 0.002647 :`B` 1.0 :`A` 1.0) :!type "LinearColor Structure")))

(fn `UserConstructionScript`
  (bind _returnvalue (`PrimitiveComponent.CreateDynamicMaterialInstance` (`self.Cylinder`) 0 "/Game/Blueprints/LED/LED_Mat.LED_Mat" "None"))
  (set `self.LED Material` _returnvalue)
  (`self.Update Material Color`))