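; Flyable drone pawn that takes control from the player via PlayerPossess, storing that pawn so the Deploy Drone input can hand control back and destroy the drone.
; Movement input drives horizontal forward, strafe and vertical flight.
; Mouse look accumulates pitch and yaw into a directly set actor rotation, while stick look uses rate-scaled controller input.
; Nodes seeding pitch and yaw from the current rotation are unconnected.
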(event `InputAxis|TurnRate`
  (params (AxisValue :type "Float (single-precision)"))
  ;[1 1 1] Stick Look
  (`self.AddControllerYawInput` (* AxisValue 45.0 (`GameplayStatics.GetWorldDeltaSeconds`))))

(event `InputAxis|Turn` :overrideparent false
  (params (AxisValue :type "Float (single-precision)"))
  ;[1 1 1] Mouse Look
  (bind _output_get (set `self.Z Yaw` (+ AxisValue (`self.Z Yaw`))))
  (`self.K2_SetActorRelativeRotation` (`KismetMathLibrary.MakeRotator` 0.0 (stale `InputAxis|LookUp` _output_get) _output_get) :!label _label))

(event `InputAxis|LookUpRate`
  (params (AxisValue :type "Float (single-precision)"))
  ;[1 1 1] Stick Look
  (`self.AddControllerPitchInput` (* AxisValue 45.0 (`GameplayStatics.GetWorldDeltaSeconds`))))

(event `InputAxis|LookUp` :overrideparent false
  (params (AxisValue :type "Float (single-precision)"))
  ;[1 1 1] Mouse Look
  (bind _output_get (set `self.Y Pitch` (+ (* -1 AxisValue) (`self.Y Pitch`))))
  (goto _label))

(event `InputAxis|MoveForward` :consume false :overrideparent false
  (params (AxisValue :type "Float (single-precision)"))
  (bind (_returnvalue_x _returnvalue_y) (`KismetMathLibrary.BreakVector` (`self.GetActorForwardVector`)))
  ;[1 1 1] Move
  (`self.AddMovementInput` (`KismetMathLibrary.MakeVector` _returnvalue_x _returnvalue_y) AxisValue))

(event `/Game/Blueprints/Possessing.Player Possess`
  (params (Player :type "/Game/Blueprints/FirstPersonCharacter Object Reference"))
  ;[1 1 1] Player Possesses Drone
  (bind _output_get (set `self.Player` Player))
  (`Controller.Possess` (`self.GetController` _output_get) self))

(event `InputAxis|MoveRight` :consume false :overrideparent false
  (params (AxisValue :type "Float (single-precision)"))
  ;[1 1 1] Move
  (`self.AddMovementInput` (`self.GetActorRightVector`) AxisValue))

(event `InputAction|Deploy Drone`
  (params (Key :type "Key Structure"))
  ;[1 1 1] Drone Possesses Player
  (:`Pressed`
    (`Controller.Possess` (`self.GetController`) (`self.Player`))
    (`self.K2_DestroyActor`)))

(event `InputAxis|Fly`
  (params (AxisValue :type "Float (single-precision)"))
  (bind (_returnvalue_x _returnvalue_y _returnvalue_z) (`KismetMathLibrary.BreakVector` (`self.GetActorUpVector`)))
  ;[1 1 1] Move
  (`self.AddMovementInput` (`KismetMathLibrary.MakeVector` 0.0 0.0 _returnvalue_z) AxisValue))

(fn `UserConstructionScript`)