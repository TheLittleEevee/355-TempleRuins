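; Interactable lever that switches a linked actor on or off when the player interacts with it.
; It acts only if that actor is valid and implements the ToggleableObject interface.
; Timelines animate the stick's roll, then on finishing send the on or off message and update IsOn.
; The construction script poses the stick to match the initial IsOn state.
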(event `/Game/Blueprints/Interfaces/PlayerCanInteract.Player Wants to Interact`
  (params (Player :type "/Game/Blueprints/FirstPersonCharacter Object Reference"))
  (bind _other_actors_controlled_by_this_actor (`self.Other Actors Controlled by this Actor`))
  (`/Engine/EditorBlueprintResources/StandardMacros.IsValid` _other_actors_controlled_by_this_actor
    (:`Is Valid`
      (if (`KismetSystemLibrary.DoesImplementInterface` _other_actors_controlled_by_this_actor "/Game/Blueprints/Interfaces/ToggleableObject.ToggleableObject_C")
        (if (`self.Is On`)
          (bind (_direction _flip_to_off) (`Timeline|Switch Off` :!via `PlayFromStart`)
            (:`Update`
              (`SceneComponent.K2_SetRelativeRotation` (`self.Stick`) (`KismetMathLibrary.MakeRotator` _flip_to_off) false false))
            (:`Finished`
              (message `/Game/Blueprints/Interfaces/ToggleableObject.Turn Off` _other_actors_controlled_by_this_actor)
              (set `self.Is On` false)))
          (else
            (bind (_direction_2 _flip_to_on) (`Timeline|Switch On` :!via `PlayFromStart`)
              (:`Update`
                (`SceneComponent.K2_SetRelativeRotation` (`self.Stick`) (`KismetMathLibrary.MakeRotator` _flip_to_on) false false))
              (:`Finished`
                (message `/Game/Blueprints/Interfaces/ToggleableObject.Turn On` _other_actors_controlled_by_this_actor)
                (set `self.Is On` true)))))))))

(fn `UserConstructionScript`
  (if (`self.Is On`)
    (`SceneComponent.K2_SetRelativeRotation` (`self.Stick`) (`KismetMathLibrary.MakeRotator` 40.0) false false)
    (else
      (`SceneComponent.K2_SetRelativeRotation` (`self.Stick`) (`KismetMathLibrary.MakeRotator` -40.0) false false))))